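; Synapse actor that carries either of the two TopDownGameMode players both ways between a start and an end neuron.
; Construction script builds spline meshes with a dynamic material and places triggers and labels at spline points 0 and 1.
; Trigger overlaps hide the player, disable collision and snap to the spline point.
; Delay loops then lerp position straight toward the opposite neuron while animating the "Anim" parameter, restoring the player on arrival.
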(event `self.ReceiveBeginPlay`
  (bind _astop_down_game_mode (cast `/Game/TopDownBP/Blueprints/TopDownGameMode` (`GameplayStatics.GetGameMode`)))
  (`KismetSystemLibrary.Delay` 0.2)
  (`GameplayStatics.GetAllActorsOfClass` "/Game/Test/BP_Spark.BP_Spark_C")
  (bind _players (`/Game/TopDownBP/Blueprints/TopDownGameMode.Players` _astop_down_game_mode))
  (bind _output_get (set `self.Player 01` (`|GetArrayItem` _players)))
  (set `self.Cube P1` (`/Game/Test/BP_Spark.Cube` _output_get))
  (bind _output_get_2 (set `self.Player 02` (`|GetArrayItem` _players 1)))
  (set `self.Cube p2` (`/Game/Test/BP_Spark.Cube` _output_get_2)))

(event `self.Start Trigger.OnComponentBeginOverlap`
  (params (OverlappedComponent :type "PrimitiveComponent Object Reference") (OtherActor :type "Actor Object Reference") (OtherComp :type "PrimitiveComponent Object Reference") (OtherBodyIndex :type Integer) (bFromSweep :type Boolean) (SweepResult :type "HitResult Structure (by ref)"))
  (bind _player_01 (`self.Player 01`))
  (bind _player_02 (`self.Player 02`))
  (bind _returnvalue (`SplineComponent.GetLocationAtSplinePoint` (`self.Spline`) 0 "World"))
  ;[1 1 1] Identité
  (if (== OtherComp (`self.Cube P1`))
    (`self.SetActorHiddenInGame` _player_01 true)
    ;[1 1 1] Coller au point 0 de la spline (START)
    (`self.SetActorEnableCollision` _player_01 false)
    (`KismetSystemLibrary.PrintString` "DISABLE" true true (struct :`R` 0.296856 :`G` 1.0 :`A` 1.0))
    (bind _output_get (set `/Game/Test/BP_Spark.Location along spline` _returnvalue _player_01))
    (`self.K2_SetActorLocation` _player_01 _output_get false false)
    (set `self.AnimationMaterial` (`self.AnimationMatStart`))
    ;[1 1 1] Loop Selon la spline
    (`self.P1 Start to End` :!label _label)
    (if (`self.P1 Start to End Done `)
      (`self.K2_SetActorLocation` _player_01 (`self.K2_GetActorLocation` (`self.BP_NeuroneEnd`)) false false)
      (`KismetSystemLibrary.Delay` 0.05)
      ;[1 1 1] Collision on
      (`self.SetActorEnableCollision` _player_01 true)
      (`PrimitiveComponent.SetCollisionEnabled` (`/Game/Test/BP_Spark.Cube` _player_01) "QueryAndPhysics")
      (`self.SetActorHiddenInGame` _player_01 false)
      (`KismetSystemLibrary.PrintString` "COMPLETE" true true (struct :`R` 1.0 :`A` 1.0) :!label _label_2)
      (else
        (`KismetSystemLibrary.Delay` 0.005)
        (goto _label)))
    (else
      (`self.SetActorHiddenInGame` _player_02 true)
      (if (== OtherComp (`self.Cube p2`))
        (`self.SetActorEnableCollision` _player_02 false)
        (bind _output_get_2 (set `/Game/Test/BP_Spark.Location along spline` _returnvalue _player_02))
        (`self.K2_SetActorLocation` _player_02 _output_get_2 false false)
        (set `self.AnimationMaterial` (`self.AnimationMatStart`))
        (`self.P2 Start to End` :!label _label_3)
        (if (`self.P2 Start to End Done`)
          (`self.K2_SetActorLocation` _player_02 (`self.K2_GetActorLocation` (`self.BP_NeuroneEnd`)) false false)
          (`KismetSystemLibrary.Delay` 0.05)
          (`self.SetActorEnableCollision` _player_02 true)
          (`PrimitiveComponent.SetCollisionEnabled` (`/Game/Test/BP_Spark.Cube` _player_02) "QueryAndPhysics")
          (`self.SetActorHiddenInGame` _player_02 false)
          (goto _label_2)
          (else
            (`KismetSystemLibrary.Delay` 0.005)
            (goto _label_3)))
        (else
          (`KismetSystemLibrary.PrintString` "JE NE SAIS PAS QUI TU ES" true true (struct :`R` 1.0 :`G` 0.327564 :`A` 1.0))
          (`KismetSystemLibrary.PrintString` (`KismetSystemLibrary.GetDisplayName` OtherComp)))))))

(event `self.End Trigger.OnComponentBeginOverlap`
  (params (OverlappedComponent :type "PrimitiveComponent Object Reference") (OtherActor :type "Actor Object Reference") (OtherComp :type "PrimitiveComponent Object Reference") (OtherBodyIndex :type Integer) (bFromSweep :type Boolean) (SweepResult :type "HitResult Structure (by ref)"))
  (bind _player_01 (`self.Player 01`))
  (bind _player_02 (`self.Player 02`))
  (bind _returnvalue (`SplineComponent.GetLocationAtSplinePoint` (`self.Spline`) 1 "World"))
  ;[1 1 1] Identité
  (if (== OtherComp (`self.Cube P1`))
    (`self.SetActorHiddenInGame` _player_01 true)
    ;[1 1 1] Coller au point 0 de la spline (START)
    (`self.SetActorEnableCollision` _player_01 false)
    (`KismetSystemLibrary.PrintString` "DISABLE" true true (struct :`R` 0.296856 :`G` 1.0 :`A` 1.0))
    (bind _output_get (set `/Game/Test/BP_Spark.Location along spline` _returnvalue _player_01))
    (`self.K2_SetActorLocation` _player_01 _output_get false false)
    (set `self.AnimationMaterial` (`self.AnimationMatEnd`))
    ;[1 1 1] Loop Selon la spline
    (`self.P1 End to Start` :!label _label_4)
    (if (`self.P1 End to Start Done`)
      (`self.K2_SetActorLocation` _player_01 (`self.K2_GetActorLocation` (`self.Bp_NeuroneStart`)) false false)
      (`KismetSystemLibrary.Delay` 0.05)
      ;[1 1 1] Collision on
      (`self.SetActorEnableCollision` _player_01 true)
      (`PrimitiveComponent.SetCollisionEnabled` (`/Game/Test/BP_Spark.Cube` _player_01) "QueryAndPhysics")
      (`self.SetActorHiddenInGame` _player_01 false)
      (`KismetSystemLibrary.PrintString` "COMPLETE" true true (struct :`R` 1.0 :`G` 0.900142 :`A` 1.0) :!label _label_5)
      (else
        (`KismetSystemLibrary.Delay` 0.005)
        (goto _label_4)))
    (elif (== OtherComp (`self.Cube p2`))
      (`self.SetActorHiddenInGame` _player_02 true)
      (`self.SetActorEnableCollision` _player_02 false)
      (bind _output_get_2 (set `/Game/Test/BP_Spark.Location along spline` _returnvalue _player_02))
      (`self.K2_SetActorLocation` _player_02 _output_get_2 false false)
      (set `self.AnimationMaterial` (`self.AnimationMatEnd`))
      (`self.P2 End to Start` :!label _label_6)
      (if (`self.P2 End to Start Done`)
        (`self.K2_SetActorLocation` _player_02 (`self.K2_GetActorLocation` (`self.Bp_NeuroneStart`)) false false)
        (`KismetSystemLibrary.Delay` 0.05)
        (`self.SetActorEnableCollision` _player_02 true)
        (`PrimitiveComponent.SetCollisionEnabled` (`/Game/Test/BP_Spark.Cube` _player_02) "QueryAndPhysics")
        (`self.SetActorHiddenInGame` _player_02 false)
        (goto _label_5)
        (else
          (`KismetSystemLibrary.Delay` 0.005)
          (goto _label_6)))
      (else
        (`KismetSystemLibrary.PrintString` "JE NE SAIS PAS QUI TU ES" true true (struct :`R` 1.0 :`G` 0.327564 :`A` 1.0))))))

(fn `P1 End to Start`
  (bind _player_01 (`self.Player 01`))
  (bind _returnvalue (`self.K2_GetActorLocation` (`self.Bp_NeuroneStart`)))
  (bind _returnvalue_2 (`KismetMathLibrary.VLerp` (`/Game/Test/BP_Spark.Location along spline` _player_01) _returnvalue (`self.AlphaVitesse`)))
  (bind _output_get (set `self.AnimationMaterial` (`KismetMathLibrary.Lerp` (`self.AnimationMaterial`) (`self.AnimationMatStart`) (`self.AlphaVitesse`))))
  (`MaterialInstanceDynamic.SetScalarParameterValue` (`self.Dynamique Material`) "Anim" _output_get)
  (`self.K2_SetActorLocation` _player_01 _returnvalue_2 false false)
  (bind _output_get_2 (set `/Game/Test/BP_Spark.Location along spline` _returnvalue_2 _player_01))
  (if (== _output_get_2 _returnvalue :`ErrorTolerance` (`self.Precision Blend`))
    (set `self.P1 End to Start Done` true)
    (else
      (set `self.P1 End to Start Done` false))))

(fn `P1 Start to End`
  (bind _player_01 (`self.Player 01`))
  (bind _returnvalue (`self.K2_GetActorLocation` (`self.BP_NeuroneEnd`)))
  (bind _returnvalue_2 (`KismetMathLibrary.VLerp` (`/Game/Test/BP_Spark.Location along spline` _player_01) _returnvalue (`self.AlphaVitesse`)))
  (bind _output_get (set `self.AnimationMaterial` (`KismetMathLibrary.Lerp` (`self.AnimationMaterial`) (`self.AnimationMatEnd`) (`self.AlphaVitesse`))))
  (`MaterialInstanceDynamic.SetScalarParameterValue` (`self.Dynamique Material`) "Anim" _output_get)
  (`self.K2_SetActorLocation` _player_01 _returnvalue_2 false false)
  (bind _output_get_2 (set `/Game/Test/BP_Spark.Location along spline` _returnvalue_2 _player_01))
  (if (== _output_get_2 _returnvalue :`ErrorTolerance` (`self.Precision Blend`))
    (set `self.P1 Start to End Done ` true)
    (else
      (set `self.P1 Start to End Done ` false))))

(fn `P2 End to Start`
  (bind _player_02 (`self.Player 02`))
  (bind _returnvalue (`self.K2_GetActorLocation` (`self.Bp_NeuroneStart`)))
  (bind _returnvalue_2 (`KismetMathLibrary.VLerp` (`/Game/Test/BP_Spark.Location along spline` _player_02) _returnvalue (`self.AlphaVitesse`)))
  (bind _output_get (set `self.AnimationMaterial` (`KismetMathLibrary.Lerp` (`self.AnimationMaterial`) (`self.AnimationMatStart`) (`self.AlphaVitesse`))))
  (`MaterialInstanceDynamic.SetScalarParameterValue` (`self.Dynamique Material`) "Anim" _output_get)
  (`self.K2_SetActorLocation` _player_02 _returnvalue_2 false false)
  (bind _output_get_2 (set `/Game/Test/BP_Spark.Location along spline` _returnvalue_2 _player_02))
  (if (== _output_get_2 _returnvalue :`ErrorTolerance` (`self.Precision Blend`))
    (set `self.P2 End to Start Done` true)
    (else
      (set `self.P2 End to Start Done` false))))

(fn `P2 Start to End`
  (bind _player_02 (`self.Player 02`))
  (bind _returnvalue (`self.K2_GetActorLocation` (`self.BP_NeuroneEnd`)))
  (bind _returnvalue_2 (`KismetMathLibrary.VLerp` (`/Game/Test/BP_Spark.Location along spline` _player_02) _returnvalue (`self.AlphaVitesse`)))
  (bind _output_get (set `self.AnimationMaterial` (`KismetMathLibrary.Lerp` (`self.AnimationMaterial`) (`self.AnimationMatEnd`) (`self.AlphaVitesse`))))
  (`MaterialInstanceDynamic.SetScalarParameterValue` (`self.Dynamique Material`) "Anim" _output_get)
  (`self.K2_SetActorLocation` _player_02 _returnvalue_2 false false)
  (bind _output_get_2 (set `/Game/Test/BP_Spark.Location along spline` _returnvalue_2 _player_02))
  (if (== _output_get_2 _returnvalue :`ErrorTolerance` (`self.Precision Blend`))
    (set `self.P2 Start to End Done` true)
    (else
      (set `self.P2 Start to End Done` false))))

(fn `UserConstructionScript`
  (bind _spline (`self.Spline`))
  (bind _start_trigger (`self.Start Trigger`))
  (bind _end_trigger (`self.End Trigger`))
  (bind _spline_2 (`self.Spline`))
  (bind _material_instance (`self.Material Instance`))
  (bind _returnvalue (`SplineComponent.GetLocationAtSplinePoint` _spline 1 "Local"))
  (bind _returnvalue_2 (`SplineComponent.GetLocationAtSplinePoint` _spline 0 "Local"))
  (bind _returnvalue_3 (- (`SplineComponent.GetNumberOfSplinePoints` (`self.Spline`)) 2))
  (bind _returnvalue_4 (+ _returnvalue_3 1))
  (for _ (range (+ _returnvalue_3 1))
    (bind _returnvalue_5 (`AddComponent|NODE_AddSplineMeshComponent-0`))
    (bind _returnvalue_6 (`KismetMaterialLibrary.CreateDynamicMaterialInstance` _material_instance _material_instance))
    (bind _output_get (set `self.Dynamique Material` _returnvalue_6))
    (`PrimitiveComponent.SetMaterial` _returnvalue_5 0 _output_get)
    (`SplineMeshComponent.SetForwardAxis` _returnvalue_5 "X" true)
    (`SceneComponent.K2_AttachToComponent` _returnvalue_5 _spline_2 "None" "KeepRelative" "KeepRelative" "KeepRelative" true)
    (`SplineMeshComponent.SetStartAndEnd` _returnvalue_5 (`SplineComponent.GetLocationAtSplinePoint` _spline_2 _returnvalue_3 "Local") (`SplineComponent.GetTangentAtSplinePoint` _spline_2 _returnvalue_3 "Local") (`SplineComponent.GetLocationAtSplinePoint` _spline_2 _returnvalue_4 "Local") (`SplineComponent.GetTangentAtSplinePoint` _spline_2 _returnvalue_4 "Local") true)
    (`SceneComponent.K2_SetRelativeLocation` _start_trigger _returnvalue_2 false false)
    (`SceneComponent.K2_SetRelativeLocation` (`self.TextStart`) (+ _returnvalue_2 (25.0 50.0 0.0)) false false)
    (`SceneComponent.SetRelativeScale3D` _start_trigger (`self.Start Trigger Scale`))
    (`SceneComponent.K2_SetRelativeLocation` _end_trigger _returnvalue false false)
    (`SceneComponent.K2_SetRelativeLocation` (`self.TextEnd`) (+ _returnvalue (-75.0 50.0 0.0)) false false)
    (`SceneComponent.SetRelativeScale3D` _end_trigger (`self.End Trigger Scale`))))