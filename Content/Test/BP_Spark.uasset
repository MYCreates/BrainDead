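; Test Blueprint that moves a Cube component around its owner's origin from controller and keyboard input.
; Both CTRL axis events share one SetRelativeLocation, scaling axis values by RadiusDéplacement on X and a fixed factor on Y.
; WASD applies a fixed local offset on press and the opposite on release, so the cube is displaced while held.
; A location reset and a 2D-position debug print are left unconnected.
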(event `InputAxis|CTRL Up/Down`
  (params (AxisValue :type "Float (single-precision)"))
  (`SceneComponent.K2_SetRelativeLocation` (`self.Cube`) (`KismetMathLibrary.MakeVector` (* AxisValue (`self.Radius Déplacement`)) (* (stale `InputAxis|CTRL Left/Right` AxisValue) 50.0)) false false :!label _label))

(event `InputAxis|CTRL Left/Right`
  (params (AxisValue :type "Float (single-precision)"))
  (goto _label))

(event `Key|W`
  (params (Key :type "Key Structure"))
  (bind _cube (`self.Cube`))
  (:`Pressed`
    (`SceneComponent.K2_AddLocalOffset` _cube (100.0 0.0 0.0) false false :!label _label_2))
  (:`Released`
    (`SceneComponent.K2_AddLocalOffset` _cube (-100.0 0.0 0.0) false false :!label _label_3)))

(event `Key|S`
  (params (Key :type "Key Structure"))
  (:`Pressed`
    (goto _label_3))
  (:`Released`
    (goto _label_2)))

(event `Key|A`
  (params (Key :type "Key Structure"))
  (bind _cube (`self.Cube`))
  (:`Pressed`
    (`SceneComponent.K2_AddLocalOffset` _cube (0.0 -100.0 0.0) false false :!label _label_4))
  (:`Released`
    (`SceneComponent.K2_AddLocalOffset` _cube (0.0 100.0 0.0) false false :!label _label_5)))

(event `Key|D`
  (params (Key :type "Key Structure"))
  (:`Pressed`
    (goto _label_5))
  (:`Released`
    (goto _label_4)))

(fn `UserConstructionScript`)