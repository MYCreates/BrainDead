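; Neuron node actor for a two-player game, showing enabled direction arrows while either player overlaps its box.
; Players come from TopDownGameMode; each entry increments that player's step count and applies their arrow material.
; An armed trap spawns particles and disables input for two seconds, but both branches stun Player01 and only Player01's entry disarms it.
; The construction script previews arrows and scales the mesh from a clamped Size.
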(event `self.ReceiveBeginPlay`
  (`self.Fleche Visible` false)
  (`KismetSystemLibrary.Delay` 0.2)
  (bind _astop_down_game_mode (cast `/Game/TopDownBP/Blueprints/TopDownGameMode` (`GameplayStatics.GetGameMode`)))
  (bind _output_get (set `self.BP_Gamemode` _astop_down_game_mode))
  (bind _players (`/Game/TopDownBP/Blueprints/TopDownGameMode.Players` _output_get))
  (set `self.Player 01` (`|GetArrayItem` _players))
  (set `self.Player 02` (`|GetArrayItem` _players 1)))

(event `self.Box.OnComponentBeginOverlap`
  (params (OverlappedComponent :type "PrimitiveComponent Object Reference") (OtherActor :type "Actor Object Reference") (OtherComp :type "PrimitiveComponent Object Reference") (OtherBodyIndex :type Integer) (bFromSweep :type Boolean) (SweepResult :type "HitResult Structure (by ref)"))
  (bind _player_01 (`self.Player 01`))
  (bind _player_01_2 (`self.Player 01`))
  (if (== OtherActor (`self.Player 01`))
    (set `self.Player 1 Step` (+ (`self.Player 1 Step`) 1))
    (if (`self.Piege Dessus ?`)
      (set `self.Piege Dessus ?` false)
      (`self.Disable Input Stun` 0 _player_01_2)
      (`KismetSystemLibrary.Delay` 2.0)
      (`self.Enable Input Stun Off` 0 _player_01_2))
    (`PrimitiveComponent.SetMaterial` (`self.Up`) 0 "/Game/Materials/Mi_Arrow01.Mi_Arrow01")
    (`PrimitiveComponent.SetMaterial` (`self.Left`) 0 "/Game/Materials/Mi_Arrow01.Mi_Arrow01")
    (`PrimitiveComponent.SetMaterial` (`self.Down`) 0 "/Game/Materials/Mi_Arrow01.Mi_Arrow01")
    (`PrimitiveComponent.SetMaterial` (`self.Right`) 0 "/Game/Materials/Mi_Arrow01.Mi_Arrow01")
    (`self.Fleche Visible` true :!label _label)
    (elif (== OtherActor (`self.Player 02`))
      (set `self.Player 2 Step` (+ (`self.Player 2 Step`) 1))
      (if (`self.Piege Dessus ?`)
        (`self.Disable Input Stun` 0 _player_01)
        (`KismetSystemLibrary.Delay` 2.0)
        (`self.Enable Input Stun Off` 0 _player_01))
      (`PrimitiveComponent.SetMaterial` (`self.Left`) 0 "/Game/Materials/Mi_Arrow02.Mi_Arrow02")
      (`PrimitiveComponent.SetMaterial` (`self.Down`) 0 "/Game/Materials/Mi_Arrow02.Mi_Arrow02")
      (`PrimitiveComponent.SetMaterial` (`self.Up`) 0 "/Game/Materials/Mi_Arrow02.Mi_Arrow02")
      (`PrimitiveComponent.SetMaterial` (`self.Right`) 0 "/Game/Materials/Mi_Arrow02.Mi_Arrow02")
      (goto _label))))

(event `self.Box.OnComponentEndOverlap`
  (params (OverlappedComponent :type "PrimitiveComponent Object Reference") (OtherActor :type "Actor Object Reference") (OtherComp :type "PrimitiveComponent Object Reference") (OtherBodyIndex :type Integer))
  (if (== OtherActor (`self.Player 01`))
    (`self.Fleche Visible` false :!label _label_2)
    (elif (== OtherActor (`self.Player 02`))
      (goto _label_2))))

(fn `Disable Input Stun`
  (params (Index :type Integer) (Player :type "/Game/Test/BP_Spark Object Reference"))
  (`self.DisableInput` Player (`GameplayStatics.GetPlayerController` Index))
  (if (== Index 0)
    (`GameplayStatics.SpawnEmitterAtLocation` "/Game/FX/PS/PS_MineDeclenche_02.PS_MineDeclenche_02" (+ (`self.K2_GetActorLocation`) (-60.0 0.0 0.0)))
    (else
      (`GameplayStatics.SpawnEmitterAtLocation` "/Game/FX/PS/PS_MineDeclenche_01.PS_MineDeclenche_01"))))

(fn `Enable Input Stun Off`
  (params (Index :type Integer) (Player :type "/Game/Test/BP_Spark Object Reference"))
  (`self.EnableInput` Player (`GameplayStatics.GetPlayerController` Index)))

(fn `Fleche Visible`
  (params (`Is Overlap ?` :type Boolean))
  (if (and (`self.Up Visible`) `Is Overlap ?`)
    (`SceneComponent.SetVisibility` (`self.Up`) true false)
    (else
      (`SceneComponent.SetVisibility` (`self.Up`) false false)))
  (if (and (`self.Down Visible`) `Is Overlap ?`)
    (`SceneComponent.SetVisibility` (`self.Down`) true false)
    (else
      (`SceneComponent.SetVisibility` (`self.Down`) false false)))
  (if (and (`self.Left Visible`) `Is Overlap ?`)
    (`SceneComponent.SetVisibility` (`self.Left`) true false)
    (else
      (`SceneComponent.SetVisibility` (`self.Left`) false false)))
  (if (and (`self.Right Visible`) `Is Overlap ?`)
    (`SceneComponent.SetVisibility` (`self.Right`) true false)
    (else
      (`SceneComponent.SetVisibility` (`self.Right`) false false))))

(fn `UserConstructionScript`
  (`self.Fleche Visible` true)
  (switch `int` (`KismetMathLibrary.Clamp` (`self.Size`) 0 2)
    (:`0`
      (`SceneComponent.SetRelativeScale3D` (`self.StaticMesh`) (0.25 0.25 0.25)))
    (:`1`
      (`SceneComponent.SetRelativeScale3D` (`self.StaticMesh`) (0.35 0.35 0.35)))
    (:`2`
      (`SceneComponent.SetRelativeScale3D` (`self.StaticMesh`) (0.45 0.45 0.45)))))