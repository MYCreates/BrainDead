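; Player character Blueprint with rudimentary movement input and debug tracing.
; MoveForward adds both controller yaw and movement along a forward vector built from control pitch used as roll, with zero yaw.
; It then draws a persistent Camera-channel line trace from player location to the raw forward vector as world endpoint, printing the hit actor and that vector.
; MoveRight is empty, with its strafe logic left disconnected.
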(event `InputAxis|MoveForward`
  (params (AxisValue :type "Float (single-precision)"))
  (bind _returnvalue (`GameplayStatics.GetPlayerCharacter` 0))
  (bind _returnvalue_2 (`self.GetActorForwardVector` _returnvalue))
  (`self.AddControllerYawInput` _returnvalue AxisValue)
  (`self.AddMovementInput` (`KismetMathLibrary.GetForwardVector` (`KismetMathLibrary.MakeRotator` (.pitch (`self.GetControlRotation`)))) AxisValue)
  (bind _outhit (`KismetSystemLibrary.LineTraceSingle` :`Start` (`self.K2_GetActorLocation` _returnvalue) :`End` _returnvalue_2 :`TraceChannel` "TraceTypeQuery2" :`DrawDebugType` "Persistent"))
  (`KismetSystemLibrary.PrintString` (`KismetSystemLibrary.GetObjectName` (`.HitActor` (`GameplayStatics.BreakHitResult` _outhit))))
  (`KismetSystemLibrary.PrintString` (`KismetStringLibrary.Conv_VectorToString` _returnvalue_2) true true (struct :`R` 1.0 :`G` 0.082387 :`B` 0.12219 :`A` 1.0)))

(event `InputAxis|MoveRight`
  (params (AxisValue :type "Float (single-precision)")))

(fn `UserConstructionScript`)