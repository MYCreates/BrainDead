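; BP_LootPickUp is a resource pickup that credits BP_Spark when that character overlaps it.
; On overlap it increments the character's NumberOfRessources and plays a sound and particle effect at the character's location.
; The pickup never destroys or disables itself, so each new overlap counts again.
; A Spawn function, not called here, creates another pickup at a random unit vector, effectively beside the world origin.
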(event `self.ReceiveActorBeginOverlap`
  (params (OtherActor :type "Actor Object Reference"))
  (bind _returnvalue (`self.K2_GetActorLocation` (`self.Charac Ref`)))
  (bind _asbp_spark (cast `/Game/Test/BP_Spark` OtherActor))
  (set `self.Charac Ref` _asbp_spark)
  (`GameplayStatics.PlaySoundAtLocation` "/Engine/EditorSounds/Notifications/CompileSuccess.CompileSuccess" _returnvalue (struct) 1.0 1.0 0.0 null null null)
  (set `/Game/Test/BP_Spark.Number of Ressources` (+ (`/Game/Test/BP_Spark.Number of Ressources` (`self.Charac Ref`)) 1) (`self.Charac Ref`))
  (`GameplayStatics.SpawnEmitterAtLocation` "/Engine/Functions/Engine_MaterialFunctions02/ExampleContent/3dParticleOpacity_Particle.3dParticleOpacity_Particle" _returnvalue))

(fn `Spawn`
  (`|SpawnActorFromClass` "BP_LootPickUp_C" (`KismetMathLibrary.MakeTransform` (`KismetMathLibrary.RandomUnitVector`)) "Undefined" "OverrideRootScale" null null))

(fn `UserConstructionScript`)