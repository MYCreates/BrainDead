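; BP_SplineSynapse is a spline-driven mesh Blueprint that, judging by its name, depicts a synapse strand.
; Its construction script adds one X-forward spline mesh component per spline segment and attaches each to the spline.
; The loop index is unused, so every component takes the last segment's local positions and tangents, stacking there instead of spanning the whole spline.
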(fn `UserConstructionScript`
  (bind _spline (`self.Spline`))
  (bind _returnvalue (- (`SplineComponent.GetNumberOfSplinePoints` (`self.Spline`)) 2))
  (bind _returnvalue_2 (+ _returnvalue 1))
  (for _ (range (+ _returnvalue 1))
    (bind _returnvalue_3 (`AddComponent|NODE_AddSplineMeshComponent-0`))
    (`SplineMeshComponent.SetForwardAxis` _returnvalue_3 "X" true)
    (`SceneComponent.K2_AttachToComponent` _returnvalue_3 _spline "None" "KeepRelative" "KeepRelative" "KeepRelative" true)
    (`SplineMeshComponent.SetStartAndEnd` _returnvalue_3 (`SplineComponent.GetLocationAtSplinePoint` _spline _returnvalue "Local") (`SplineComponent.GetTangentAtSplinePoint` _spline _returnvalue "Local") (`SplineComponent.GetLocationAtSplinePoint` _spline _returnvalue_2 "Local") (`SplineComponent.GetTangentAtSplinePoint` _spline _returnvalue_2 "Local") true)))